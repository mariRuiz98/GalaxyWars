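; BP_SSPawn is the player ship pawn for a space shooter, handling Enhanced Input movement and firing.
; BeginPlay adds the input mapping context, and move events save the 2D input or zero it on release.
; Tick moves the ship without sweep from that input and Speed, along world right and actor forward.
; The fire action calls DoFire, which spawns the Ammo class at FirePoint's transform.
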(event Input|EnhancedActionEvents|EnhancedInputActionBP_InputFire
  (params (ActionValue :type Boolean) (ElapsedSeconds :type Float%20%28double-precision%29) (TriggeredSeconds :type Float%20%28double-precision%29) (InputAction :type Input%20Action%20Object%20Reference :default "/Game/00_SpaceShooter/Input/BP_InputFire.BP_InputFire"))
  (:Started
    (CallFunction|DoFire)))

(event Input|EnhancedActionEvents|EnhancedInputActionBP_InputMove
  (params (ActionValue :type Vector%202D%20Structure) (ElapsedSeconds :type Float%20%28double-precision%29) (TriggeredSeconds :type Float%20%28double-precision%29) (InputAction :type Input%20Action%20Object%20Reference :default "/Game/00_SpaceShooter/Input/BP_InputMove.BP_InputMove"))
  (:Triggered
    (Variables|Default|SetInputSaved ActionValue))
  (:Canceled
    (Variables|Default|SetInputSaved "" :!label _label))
  (:Completed
    (goto _label)))

(event EventBeginPlay
  ;[1 1 1] Inputs Player Control
  (bind _asplayer_controller (Utilities|Casting|CastToPlayerController (Pawn|GetController)))
  (Utilities|IsValid (PlayerController|LocalPlayerSubsystems|GetEnhancedInputLocalPlayerSubsystem _asplayer_controller)
    (:Is%20Valid
      (Input|AddMappingContext (PlayerController|LocalPlayerSubsystems|GetEnhancedInputLocalPlayerSubsystem _asplayer_controller) "/Game/00_SpaceShooter/Input/BP_InputMapping.BP_InputMapping" 0 "(bIgnoreAllPressedKeysUntilRelease=True,bForceImmediately=False,bNotifyUserSettings=False)"))))

(event Collision|EventActorBeginOverlap
  (params (OtherActor :type Actor%20Object%20Reference)))

(event EventTick
  (params (DeltaSeconds :type Float%20%28single-precision%29))
  (bind _speed (Variables|Default|GetSpeed))
  (bind _inputsaved (Variables|Default|GetInputSaved))
  (bind _returnvalue (* DeltaSeconds _speed))
  ;[1 1 1] Manage Space Ship Movement
  (Transformation|SetActorLocation (+ (+ (* (Math|Vector|GetRightVector "0, 0, 0") (* _returnvalue (.x _inputsaved))) (* (* _returnvalue (.y _inputsaved)) (Transformation|GetActorForwardVector))) (Transformation|GetActorLocation)) false false))

(fn ConstructionScript)

(fn DoFire
  (Game|SpawnActorfromClass (Variables|Default|GetAmmo) (Transformation|GetWorldTransform (Variables|Default|GetFirePoint)) "Undefined" "MultiplyWithRoot" 0 0))